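; Elevator actor whose platform travels vertically between its start height and MaxHeight, which can be derived on BeginPlay from the cable start and end points.
; SetMoveState switches between up, down and stay, looping or stopping the platform animation.
; Tick moves the platform, offsets the cable through a material parameter to match, and stops at either limit.
; The construction script links the child lever to this elevator and sizes an arrow to the travel height.
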(event `self.ReceiveBeginPlay`
  (bind (_returnvalue_x _returnvalue_y _returnvalue_z) (`KismetMathLibrary.BreakVector` (`SceneComponent.K2_GetComponentLocation` (`self.CableEndPoint`))))
  (bind (_returnvalue_x_2 _returnvalue_y_2 _returnvalue_z_2) (`KismetMathLibrary.BreakVector` (`SceneComponent.K2_GetComponentLocation` (`self.CableStartPoint`))))
  (if (`self.bDetermineMaxHeightOnBeginPlay`)
    (set `self.MaxHeight` (- _returnvalue_z_2 _returnvalue_z))))

(event `self.ReceiveTick`
  (params (DeltaSeconds :type "Float (single-precision)"))
  (bind (_relativelocation_x _relativelocation_y _relativelocation_z) (`KismetMathLibrary.BreakVector` (`SceneComponent.RelativeLocation` (`self.PlatformSkel`))))
  (bind _returnvalue (`KismetMathLibrary.FClamp` (+ _relativelocation_z (* (select `/Game/ElevatorBP/Blueprints/ElevatorStates` (`self.CurMoveState`) :`NewEnumerator0` 1.0 :`NewEnumerator1` -1.0 :!type "Float (single-precision)") DeltaSeconds (`self.Speed`))) 0.0 (`self.MaxHeight`)))
  (if (`|EnumInequality` (`self.CurMoveState`) "NewEnumerator2")
    (`MeshComponent.SetVectorParameterValueOnMaterials` (`self.Cable`) "Offset" (`KismetMathLibrary.MakeVector` 0.0 0.0 (* _returnvalue -1.0)))
    (`SceneComponent.K2_SetRelativeLocation` (`self.PlatformSkel`) (`KismetMathLibrary.MakeVector` 0.0 0.0 _returnvalue) false false)
    (if (or (== _returnvalue 0.0) (== _returnvalue (`self.MaxHeight`)))
      (`self.SetMoveState` "NewEnumerator2"))))

(fn `IsOnTop`
  (returns (ReturnValue :type Boolean))
  (bind (_relativelocation_x _relativelocation_y _relativelocation_z) (`KismetMathLibrary.BreakVector` (`SceneComponent.RelativeLocation` (`self.PlatformSkel`))))
  (return (<= (`KismetMathLibrary.Abs` (- _relativelocation_z (`self.MaxHeight`))) 10.0)))

(fn `SetMoveState`
  (params (NewMoveState :type "/Game/ElevatorBP/Blueprints/ElevatorStates Enum" :default "NewEnumerator0"))
  (bind _output_get (set `self.CurMoveState` NewMoveState))
  (switch `/Game/ElevatorBP/Blueprints/ElevatorStates` _output_get
    (:`NewEnumerator0`
      (`SkeletalMeshComponent.PlayAnimation` (`self.PlatformSkel`) "/Game/ElevatorBP/Meshes/PlatformRig_Anim.PlatformRig_Anim" true :!label _label))
    (:`NewEnumerator1`
      (goto _label))
    (:`NewEnumerator2`
      (`SkeletalMeshComponent.Stop` (`self.PlatformSkel`)))))

(fn `UserConstructionScript`
  (bind _arrow (`self.Arrow`))
  (`parent.UserConstructionScript`)
  (`|ExecutionSequence`
    (:`then_0`
      (bind _asbp_elevator_lever (cast `/Game/ElevatorBP/Blueprints/BP_ElevatorLever` (`ChildActorComponent.ChildActor` (`self.Lever`))))
      (set `/Game/ElevatorBP/Blueprints/BP_ElevatorLever.ElevatorRef` self _asbp_elevator_lever)
      (`SceneComponent.K2_SetWorldLocation` _arrow (`SceneComponent.K2_GetComponentLocation` (`self.PlatformSkel`)) false false)
      (set `ArrowComponent.ArrowLength` (`self.MaxHeight`) _arrow))))