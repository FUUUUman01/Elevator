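; Elevator lever Blueprint that controls the movement state of a referenced elevator.
; ActivateLever plays a one-shot animation on the lever's skeletal mesh, then calls SetMoveState on ElevatorRef if it is valid.
; From the third, apparently idle, move state it picks a travel state based on IsOnTop; otherwise it toggles between the two travel states, reversing the elevator.
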(event `ActivateLever`
  (`SkeletalMeshComponent.PlayAnimation` (`self.LeverSkel`) "/Game/ElevatorBP/Meshes/LeverRig_Anim.LeverRig_Anim" false)
  (bind _elevatorref (`self.ElevatorRef`)
    (:`then`
      (if (`|EnumEquality` (`/Game/ElevatorBP/Blueprints/BP_Elevator.CurMoveState` _elevatorref) "NewEnumerator2")
        (`/Game/ElevatorBP/Blueprints/BP_Elevator.SetMoveState` (`self.ElevatorRef`) (select `bool` (`/Game/ElevatorBP/Blueprints/BP_Elevator.IsOnTop` (`self.ElevatorRef`)) :`false` "NewEnumerator0" :`true` "NewEnumerator1" :!type "/Game/ElevatorBP/Blueprints/ElevatorStates Enum"))
        (else
          (`/Game/ElevatorBP/Blueprints/BP_Elevator.SetMoveState` (`self.ElevatorRef`) (select `bool` (`|EnumEquality` (`/Game/ElevatorBP/Blueprints/BP_Elevator.CurMoveState` (`self.ElevatorRef`)) "NewEnumerator0") :`false` "NewEnumerator0" :`true` "NewEnumerator1" :!type "/Game/ElevatorBP/Blueprints/ElevatorStates Enum")))))
    (:`else`)))

(fn `UserConstructionScript`)